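; Child enemy Blueprint that handles being targeted and being executed.
; Targeting sets an overlay material on the mesh as a highlight, and ending the target clears it.
; On execution it turns yaw-only toward the executor, sets a Motion Warping target at its own location with that rotation, plays the indexed reaction montage and marks itself dead.
; A getter exposes the alive state.
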(event `OnTargeted`
  (`MeshComponent.SetOverlayMaterial` (`self.Mesh`) "/Game/Blueprints/Character/BattleMage/AbilityTestMaterial/M_Overlay_Inst.M_Overlay_Inst"))

(event `EndTarget`
  (`MeshComponent.SetOverlayMaterial` (`self.Mesh`) null))

(event `Executed`
  (params (Target :type "Actor Object Reference") (ExecIndex :type Integer))
  (bind (_returnvalue_roll _returnvalue_pitch) (`KismetMathLibrary.BreakRotator` (`self.K2_GetActorRotation`)))
  (bind (_returnvalue_roll_2 _returnvalue_pitch_2 _returnvalue_yaw) (`KismetMathLibrary.BreakRotator` (`KismetMathLibrary.FindLookAtRotation` (`self.K2_GetActorLocation`) (`self.K2_GetActorLocation` Target))))
  (bind _returnvalue (`KismetMathLibrary.MakeRotator` _returnvalue_roll _returnvalue_pitch _returnvalue_yaw))
  (`self.K2_SetActorRotation` _returnvalue)
  (`MotionWarpingComponent.AddOrUpdateWarpTargetFromLocationAndRotation` (`self.MotionWarping`) "Target" (`self.K2_GetActorLocation`) _returnvalue)
  (`self.PlayAnimMontage` (`|GetArrayItem` (`self.ExecReactionMontage`) ExecIndex))
  (set `self.bIsAlive` false))

(fn `IsAlive?`
  (returns (ReturnValue :type Boolean))
  (return (`self.bIsAlive`)))

(fn `UserConstructionScript`
  (`parent.UserConstructionScript`))