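; Charge attack gameplay ability that separates a tap from a held charge on an avatar implementing CombatInterface.
; On activation it fires a charge cue and plays a looping power-attack montage, whose gameplay event sets the charge-loop state and disables movement.
; In parallel, input release before MinChargeTime restores walking, clears that state and plays a run attack before ending.
; A longer hold just ends the ability, leaving the montage running.
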(event `self.K2_ActivateAbility`
  (`self.ImplementsInterface`)
  (`self.StoreOwnerVariables`)
  (`|ExecutionSequence`
    (:`then_0`
      (`self.K2_ExecuteGameplayCue` (struct :`TagName` "GameplayCue.ChargeLoop"))
      (`AbilityTask_PlayMontageAndWait.CreatePlayMontageAndWaitProxy` "None" "/Game/Power_Attack_Loop_Seq2_Montage1.Power_Attack_Loop_Seq2_Montage1" 1.0 "None" false
        (:`then`
          (`AbilityTask_WaitGameplayEvent.WaitGameplayEvent` (struct :`TagName` "Event.Montage.Charge") null true
            (:`EventReceived`
              (`self.ChargeLoop`))))))
    (:`then_1`
      (bind (_asynctaskproxy _timeheld) (`AbilityTask_WaitInputRelease.WaitInputRelease` false)
        (:`OnRelease`
          (set `self.Time Held` _timeheld)
          (if (> (`self.MinChargeTime`) (`self.Time Held`))
            (`CharacterMovementComponent.SetMovementMode` (`Character.CharacterMovement` (`self.OwnerCharacter`)) "MOVE_Walking" 0)
            (message `CombatInterface.SetInChargeLoop` (`self.GetAvatarActorFromActorInfo`) false)
            (`AbilityTask_PlayMontageAndWait.CreatePlayMontageAndWaitProxy` "None" "/Game/Run_Attack_01_Seq2_Montage.Run_Attack_01_Seq2_Montage" 1.0 "None" false
              (:`OnCompleted`
                (`self.K2_EndAbility`)))
            (else
              (`self.K2_EndAbility`))))))))

(event `self.K2_OnEndAbility`
  (params (bWasCancelled :type Boolean)))

(fn `ChargeLoop`
  (message `CombatInterface.SetInChargeLoop` (`self.GetAvatarActorFromActorInfo`) true)
  (`CharacterMovementComponent.DisableMovement` (`Character.CharacterMovement` (`self.OwnerCharacter`))))

(fn `GetCombatSocketLocation`
  (params (MontageTag :type "GameplayTag Structure (by ref)"))
  (returns (ReturnValue :type "Vector Structure"))
  (return (0.0 0.0 0.0)))

(fn `GetHitReactMontage`
  (returns (ReturnValue :type "AnimMontage Object Reference"))
  (return null))

(fn `GetPlayerLevel`
  (returns (ReturnValue :type Integer))
  (return 0))

(fn `ImplementsInterface`
  (if (not (`KismetSystemLibrary.DoesImplementInterface` (`self.GetAvatarActorFromActorInfo`) "/Script/BattleMage.CombatInterface"))
    (`self.K2_EndAbility`)))