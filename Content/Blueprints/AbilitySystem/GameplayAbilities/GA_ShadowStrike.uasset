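; Shadow Strike gameplay ability that slows time and teleports the player next to a target pawn.
; On activation it stores mouse target and owner data, drops time dilation and sphere-traces from the camera, using a facing dot product to set HitFromBehind.
; Releasing input before MinChargeTime turns the player toward a valid TargetActor and places them in front or behind it.
; Longer holds have no action, and the execution montage is unconnected.
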(event `self.K2_ActivateAbility`
  (bind _targetactor (`self.TargetActor`))
  (bind (_returnvalue_roll _returnvalue_pitch) (`KismetMathLibrary.BreakRotator` (`Actor.K2_GetActorRotation` (`self.OwnerPlayerCharacter`))))
  (bind _cameracomponent (`BMCharacter.CameraComponent` (`self.OwnerPlayerCharacter`)))
  (bind _returnvalue (`SceneComponent.K2_GetComponentLocation` _cameracomponent))
  (bind (_returnvalue_roll_2 _returnvalue_pitch_2 _returnvalue_yaw) (`KismetMathLibrary.BreakRotator` (`KismetMathLibrary.FindLookAtRotation` (`Actor.K2_GetActorLocation` (`self.OwnerPlayerCharacter`)) (`Actor.K2_GetActorLocation` (`self.TargetActor`)))))
  (bind (_asynctaskproxy _datahandle) (`TargetDataUnderMouse.CreateTargetDataUnderMouse`)
    (:`ValidData`
      (`self.StoreMouseDataInfo` (`AbilitySystemBlueprintLibrary.GetHitResultFromTargetData` _datahandle))
      (`self.StoreOwnerVariables`)
      (`|ExecutionSequence`
        (:`then_0`
          (`GameplayStatics.SetGlobalTimeDilation` 0.1)
          (bind (_outhit _returnvalue_2) (`KismetSystemLibrary.SphereTraceSingleForObjects` :`Start` _returnvalue :`End` (+ _returnvalue (* (`SceneComponent.GetForwardVector` _cameracomponent) 2000.0)) :`Radius` 15.0 :`ObjectTypes` (`|MakeArray` "ObjectTypeQuery3" :!type "EObjectTypeQuery Enum") :`DrawDebugType` "Persistent"))
          (if _returnvalue_2
            (bind (_bblockinghit _binitialoverlap _time _distance _location _impactpoint _normal _impactnormal _physmat _hitactor) (`GameplayStatics.BreakHitResult` _outhit))
            (`/Engine/EditorBlueprintResources/StandardMacros.IsValid` _hitactor
              (:`Is Valid`
                (if (!= (`self.TargetActor`) _hitactor)
                  (set `self.HitFromBehind` (`KismetMathLibrary.InRange_FloatFloat` (`Actor.GetDotProductTo` _hitactor (`self.OwnerPlayerCharacter`)) -0.1))
                  (else
                    (`GameplayStatics.SetGlobalTimeDilation` 1.0)
                    (`self.K2_EndAbility`))))
              (:`Is Not Valid`
                (`GameplayStatics.SetGlobalTimeDilation` 1.0)
                (`self.K2_EndAbility`)))
            (else
              (set `self.TargetActor` null))))
        (:`then_1`
          (bind (_asynctaskproxy_2 _timeheld) (`AbilityTask_WaitInputRelease.WaitInputRelease` false)
            (:`OnRelease`
              ;[1 1 1] MinTImeHeld
              (set `self.Time Held` _timeheld)
              (if (< (`self.Time Held`) (`self.MinChargeTime`))
                (if (`KismetSystemLibrary.IsValid` (`self.TargetActor`))
                  (`GameplayStatics.SetGlobalTimeDilation` 1.0)
                  (`Actor.K2_SetActorRotation` (`self.OwnerPlayerCharacter`) (`KismetMathLibrary.MakeRotator` _returnvalue_roll _returnvalue_pitch _returnvalue_yaw) false)
                  (`Actor.K2_SetActorLocation` (`self.OwnerPlayerCharacter`) (+ (* (`Actor.GetActorForwardVector` _targetactor) (`KismetMathLibrary.SelectFloat` 100.0 -100.0 (`self.HitFromBehind`))) (`Actor.K2_GetActorLocation` _targetactor)) false true)
                  (`self.K2_EndAbility`)
                  (else
                    (`self.K2_EndAbility`)))))))))))